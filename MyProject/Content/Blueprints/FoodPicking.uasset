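; FoodPicking is a Blueprint that keeps a running count of picked food, shown as berries.
; AddFood and RemoveFood raise or lower PickedFood by one, then pass the new total to Berrycount through UpdateBerryCount.
; Neither function checks bounds, and the event graph holds no logic.
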(event EventBeginPlay)

(event EventTick
  (params (DeltaSeconds :type Float%20%28single-precision%29)))

(fn AddFood
  (bind _result (Math|Integer|IncrementInt (Variables|Default|GetPickedFood))
    (:%20%20
      (Variables|Default|SetPickedFood _result)
      (Default|UpdateBerryCount (Variables|Default|Getberrycount) (Variables|Default|GetPickedFood)))))

(fn RemoveFood
  (bind _result (Math|Integer|DecrementInt (Variables|Default|GetPickedFood))
    (:%20%20
      (Variables|Default|SetPickedFood _result)
      (Default|UpdateBerryCount (Variables|Default|Getberrycount) (Variables|Default|GetPickedFood)))))